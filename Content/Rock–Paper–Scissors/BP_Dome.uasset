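; BP_Dome is a dome actor in a Rock–Paper–Scissors game that shows the round result through its color.
; On BeginPlay it creates a dynamic material instance on its mesh and caches the Rock-Paper-Scissors widget from the hand-tracking player pawn, though that reference goes unused.
; SetColor switches on the result to set the Color parameter: green for win, red for loss, black for draw, gray otherwise.
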(event Custom|Set%20Color
  (params (Selection :type String))
  (switch string Selection
    (:Default
      (Rendering|Material|SetVectorParameterValue (Variables|Default|GetMID) "Color" "(R=0.552083,G=0.552083,B=0.552083,A=0.000000)" :!class /Script/Engine.MaterialInstanceDynamic))
    (:Draw
      (Rendering|Material|SetVectorParameterValue :self (Variables|Default|GetMID) :ParameterName "Color" :!class /Script/Engine.MaterialInstanceDynamic))
    (:Win
      (Rendering|Material|SetVectorParameterValue (Variables|Default|GetMID) "Color" "(R=0.000000,G=1.000000,B=0.019875,A=1.000000)" :!class /Script/Engine.MaterialInstanceDynamic))
    (:Lose
      (Rendering|Material|SetVectorParameterValue (Variables|Default|GetMID) "Color" "(R=1.000000,G=0.000000,B=0.000000,A=1.000000)" :!class /Script/Engine.MaterialInstanceDynamic))))

(event EventBeginPlay
  (bind _sm_dome (Variables|Default|GetSM_Dome))
  (bind _returnvalue (Rendering|Material|CreateDynamicMaterialInstance _sm_dome 0 (Rendering|Material|GetMaterial _sm_dome 0) "None" :!class /Script/Engine.PrimitiveComponent))
  (Variables|Default|SetMID _returnvalue)
  (bind _ashand_track_verse (Utilities|Casting|CastToHand_track_Verse (Game|Player|GetPlayerPawn 0)))
  (bind _asw_rock_paper_scissors (Utilities|Casting|CastToW_RockPaperScissors (UserInterface|GetWidget (Variables|/Game/Rock–Paper–Scissors/Hand_track_Verse.Hand_track_Verse_C|GetWidget _ashand_track_verse))))
  (Variables|Default|SetAs%20W%20Rock%20Paper%20Scissors _asw_rock_paper_scissors))

(event Collision|EventActorBeginOverlap
  (params (OtherActor :type Actor%20Object%20Reference)))

(event EventTick
  (params (DeltaSeconds :type Float%20%28single-precision%29)))

(fn ConstructionScript)