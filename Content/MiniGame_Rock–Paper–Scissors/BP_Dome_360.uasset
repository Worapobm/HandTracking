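; 360 dome actor for the Rock-Paper-Scissors minigame that plays looping media for lobby, idle, action, round results, victory and game over.
; Game events scan the DTMedia table by media type, with idle and result clips also matched to BotState.
; SetSummary tallies rounds and wins, advances BotState on player wins and picks the result clip.
; PlayMediaSourceLoop plays through the media player, reopening the current source when it ends.
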(event Custom|Set%20Summary
  (params (Selection :type String))
  ;[0.8177 0.1278 0.1278 0.5] Summary
  (Variables|Default|SetbCloseGate false)
  (bind _output_get (Variables|Default|SetSum Selection))
  (switch string _output_get
    (:Draw
      (Math|Integer|IncrementInt (Variables|Default|GetRound)
        (:%20%20
          (for _array_element (Variables|Default|GetAll%20Row%20Name) :!label _label
            (bind _returnvalue (Utilities|GetDataTableRow (Variables|Default|GetDT_Media) _array_element)
              (:then
                (switch Utilities|FlowControl|Switch|SwitchonE_MediaType (.MediaType (Utilities|Struct|BreakST_Data_Media _returnvalue))
                  (:NewEnumerator0
                    _)
                  (:NewEnumerator1
                    _)
                  (:NewEnumerator6
                    _))
                (bind (_output_current_media _output_media_source _finish) (CallFunction|PlayMediawithGameCondition (.MediaSource (Utilities|Struct|BreakST_Data_Media _returnvalue)) (.MediaType (Utilities|Struct|BreakST_Data_Media _returnvalue)) (.Round (Utilities|Struct|BreakST_Data_Media _returnvalue))))
                (if _finish
                  (CallFunction|PlayMediaSourceLoop (Utilities|String|EnumtoString _output_current_media) _output_media_source))))))))
    (:Win
      (Math|Integer|IncrementInt (Variables|Default|GetBotState)
        (:%20%20
          (Math|Integer|IncrementInt (Variables|Default|GetPlayerWin)
            (:%20%20
              (Math|Integer|IncrementInt (Variables|Default|GetRound)
                (:%20%20
                  (goto _label))))))))
    (:Lose
      (Math|Integer|IncrementInt (Variables|Default|GetBotWin)
        (:%20%20
          (Math|Integer|IncrementInt (Variables|Default|GetRound)
            (:%20%20
              (goto _label))))))
    (:Gameover
      (Variables|Default|SetRound 0)
      (Variables|Default|SetPlayerWin 0)
      (Variables|Default|SetBotWin 0)
      (Variables|Default|SetBotState 0))))

(event Custom|Play%20Media%20Source%20Loop
  (params (Media%20Mode :type String) (Input%20Media%20Source :type Media%20Source%20Object%20Reference))
  (bind _mp (Variables|Default|GetMP))
  ;[0.8073 0.8073 0.8073 0.5] Event Play Media Source Loop
  (Variables|Default|SetMedia%20Mode Media%20Mode)
  (Media|MediaPlayer|OpenSource _mp Input%20Media%20Source)
  (EventDispatchers|AssignOnMediaOpened _mp (delegate Custom|OnMediaOpened)))

(event Custom|Play%20Victory
  (params (Sum :type String))
  ;[0.07541 0.8385 0.7717 0.5] Play Summary Media
  (Variables|Default|SetSum Sum)
  (for _array_element (Variables|Default|GetAll%20Row%20Name)
    (bind _returnvalue (Utilities|GetDataTableRow (Variables|Default|GetDT_Media) _array_element)
      (:then
        (switch Utilities|FlowControl|Switch|SwitchonE_MediaType (.MediaType (Utilities|Struct|BreakST_Data_Media _returnvalue))
          (:NewEnumerator10
            _)
          (:NewEnumerator7
            _))
        (if (Utilities|Enum|Equal(Enum) (Variables|Default|GetSum) (Utilities|String|EnumtoString (.MediaType (Utilities|Struct|BreakST_Data_Media _returnvalue))))
          (bind _output_get (Variables|Default|SetCurrent%20Mode (.MediaType (Utilities|Struct|BreakST_Data_Media _returnvalue))))
          (bind _output_get_2 (Variables|Default|SetCurrent%20Media%20Source (.MediaSource (Utilities|Struct|BreakST_Data_Media _returnvalue))))
          (CallFunction|PlayMediaSourceLoop (Utilities|String|EnumtoString _output_get) _output_get_2))))))

(event Custom|Game%20Over
  (params (Sum :type String))
  ;[0.07541 0.8385 0.7717 0.5] Play Summary Media
  (Variables|Default|SetSum Sum)
  (for _array_element (Variables|Default|GetAll%20Row%20Name)
    (bind _returnvalue (Utilities|GetDataTableRow (Variables|Default|GetDT_Media) _array_element)
      (:then
        (switch Utilities|FlowControl|Switch|SwitchonE_MediaType (.MediaType (Utilities|Struct|BreakST_Data_Media _returnvalue))
          (:NewEnumerator10
            _)
          (:NewEnumerator7
            _))
        (if (Utilities|Enum|Equal(Enum) (Variables|Default|GetSum) (Utilities|String|EnumtoString (.MediaType (Utilities|Struct|BreakST_Data_Media _returnvalue))))
          (bind _output_get (Variables|Default|SetCurrent%20Mode (.MediaType (Utilities|Struct|BreakST_Data_Media _returnvalue))))
          (bind _output_get_2 (Variables|Default|SetCurrent%20Media%20Source (.MediaSource (Utilities|Struct|BreakST_Data_Media _returnvalue))))
          (CallFunction|PlayMediaSourceLoop (Utilities|String|EnumtoString _output_get) _output_get_2))))))

(event Custom|ReMatch
  ;[0.279 0.3985 0.6302 0.5] Init Media Data & Play Lobby Media
  (for _array_element (stale EventBeginPlay _output_get)
    (bind _returnvalue (Utilities|GetDataTableRow (Variables|Default|GetDT_Media) _array_element)
      (:then
        (switch Utilities|FlowControl|Switch|SwitchonE_MediaType (.MediaType (Utilities|Struct|BreakST_Data_Media _returnvalue))
          (:NewEnumerator5
            (bind _output_get (Variables|Default|SetCurrent%20Mode (.MediaType (Utilities|Struct|BreakST_Data_Media _returnvalue))))
            (bind _output_get_2 (Variables|Default|SetCurrent%20Media%20Source (.MediaSource (Utilities|Struct|BreakST_Data_Media _returnvalue))))
            (CallFunction|PlayMediaSourceLoop (Utilities|String|EnumtoString _output_get) _output_get_2)))))))

(event Custom|OnEndReached_Event
  (bind _current_media_source (Variables|Default|GetCurrent%20Media%20Source))
  ;[0.8073 0.8073 0.8073 0.5] Event Play Media Source Loop
  (Media|MediaPlayer|OpenSource (Variables|Default|GetMP) _current_media_source)
  (CallFunction|PlayMediaSourceLoop (Variables|Default|GetMedia%20Mode) _current_media_source))

(event Custom|Play%20Action%20Media
  ;[0.5417 0.4274 0.1439 0.5] Play Action Media
  (for _array_element (Variables|Default|GetAll%20Row%20Name)
    (bind _returnvalue (Utilities|GetDataTableRow (Variables|Default|GetDT_Media) _array_element)
      (:then
        (switch Utilities|FlowControl|Switch|SwitchonE_MediaType (.MediaType (Utilities|Struct|BreakST_Data_Media _returnvalue))
          (:NewEnumerator4
            (bind _output_get (Variables|Default|SetCurrent%20Mode (.MediaType (Utilities|Struct|BreakST_Data_Media _returnvalue))))
            (bind _output_get_2 (Variables|Default|SetCurrent%20Media%20Source (.MediaSource (Utilities|Struct|BreakST_Data_Media _returnvalue))))
            (CallFunction|PlayMediaSourceLoop (Utilities|String|EnumtoString _output_get) _output_get_2)))))))

(event Custom|Return%20Idle
  ;[0.2955 0.4948 0.2732 0.5] Play Idle Media
  (for _array_element (Variables|Default|GetAll%20Row%20Name)
    (bind _returnvalue (Utilities|GetDataTableRow (Variables|Default|GetDT_Media) _array_element)
      (:then
        (switch Utilities|FlowControl|Switch|SwitchonE_MediaType (.MediaType (Utilities|Struct|BreakST_Data_Media _returnvalue))
          (:NewEnumerator9
            (if (== (.Round (Utilities|Struct|BreakST_Data_Media _returnvalue)) (Variables|Default|GetBotState))
              (bind _output_get (Variables|Default|SetCurrent%20Mode (.MediaType (Utilities|Struct|BreakST_Data_Media _returnvalue))))
              (bind _output_get_2 (Variables|Default|SetCurrent%20Media%20Source (.MediaSource (Utilities|Struct|BreakST_Data_Media _returnvalue))))
              (CallFunction|PlayMediaSourceLoop (Utilities|String|EnumtoString _output_get) _output_get_2))))))))

(event Custom|OnMediaOpened
  (params (OpenedUrl :type String))
  (bind _mp (Variables|Default|GetMP))
  ;[0.8073 0.8073 0.8073 0.5] Event Play Media Source Loop
  (if (Variables|Default|GetbPlay)
    (Media|MediaPlayer|Play _mp :!class /Script/MediaAssets.MediaPlayer)
    (EventDispatchers|AssignOnEndReached _mp (delegate Custom|OnEndReached_Event))))

(event EventBeginPlay
  (bind _sm_dome (Variables|Default|GetSM_Dome))
  (Utilities|FlowControl|Sequence
    (:then_0
      ;[0.279 0.3985 0.6302 0.5] Init Media Data & Play Lobby Media
      (bind _outrownames (DataTable|GetDataTableRowNames (Variables|Default|GetDT_Media)))
      (bind _output_get (Variables|Default|SetAll%20Row%20Name _outrownames))
      (for _array_element _output_get
        (bind _returnvalue (Utilities|GetDataTableRow (Variables|Default|GetDT_Media) _array_element)
          (:then
            (switch Utilities|FlowControl|Switch|SwitchonE_MediaType (.MediaType (Utilities|Struct|BreakST_Data_Media _returnvalue))
              (:NewEnumerator5
                (bind _output_get_2 (Variables|Default|SetCurrent%20Mode (.MediaType (Utilities|Struct|BreakST_Data_Media _returnvalue))))
                (bind _output_get_3 (Variables|Default|SetCurrent%20Media%20Source (.MediaSource (Utilities|Struct|BreakST_Data_Media _returnvalue))))
                (CallFunction|PlayMediaSourceLoop (Utilities|String|EnumtoString _output_get_2) _output_get_3)))))))
    (:then_1
      (bind _returnvalue_2 (Rendering|Material|CreateDynamicMaterialInstance _sm_dome 0 (Rendering|Material|GetMaterial _sm_dome 0) "None" :!class /Script/Engine.PrimitiveComponent))
      (Variables|Default|SetMID _returnvalue_2))))

(event Collision|EventActorBeginOverlap
  (params (OtherActor :type Actor%20Object%20Reference)))

(event EventTick
  (params (DeltaSeconds :type Float%20%28single-precision%29)))

(fn ConstructionScript)

(fn GetPlay
  (return (Variables|Default|GetbPlay)))

(fn SetPlay
  (params (NewValue :type Boolean))
  (Variables|Default|SetbPlay NewValue))

(fn PlayMediawithGameCondition
  (params (Current%20Media%20Source :type Media%20Source%20Object%20Reference) (Current%20Mode :type E_MediaType%20Enum :default "NewEnumerator0") (Input%20State :type Integer))
  (bind _returnvalue (Utilities|String|EnumtoString Current%20Mode))
  (bind _sum (Variables|Default|GetSum))
  (bind _botstate (Variables|Default|GetBotState))
  (bind _returnvalue_2 (Utilities|Enum|Equal(Enum) _sum _returnvalue))
  (bind _returnvalue_3 (== Input%20State _botstate))
  (switch string _sum
    (:Draw
      (if _returnvalue_2
        (bind _output_get (Variables|Default|SetCurrent%20Mode Current%20Mode :!label _label))
        (bind _output_get_2 (Variables|Default|SetCurrent%20Media%20Source Current%20Media%20Source))
        (return _output_get _output_get_2 _returnvalue_3)))
    (:Win
      (if _returnvalue_2 :!label _label_2
        (if _returnvalue_3
          (goto _label))))
    (:Lose
      (goto _label_2))))