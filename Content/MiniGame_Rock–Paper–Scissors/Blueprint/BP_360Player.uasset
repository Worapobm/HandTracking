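; BP_360Player is a media playback actor in the Rock-Paper-Scissors minigame, apparently for 360 video, that plays and loops a media source.
; PlayMedia stores the source, opens it on the MP media player and binds the opened event, which starts playback when Play is set.
; At end of media it reopens the stored source and calls PlayMediaSourceLoop, which re-enters the PlayMedia chain and binds the opened event again.
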(event Custom|OnEndReached_Event
  (bind _current_media_source (Variables|Default|GetCurrent%20Media%20Source))
  (Media|MediaPlayer|OpenSource (Variables|Default|GetMP) _current_media_source)
  (CallFunction|PlayMediaSourceLoop (Variables|Default|GetMedia%20Mode) _current_media_source))

(event Custom|Play%20Media%20Source%20Loop
  (params (Media%20Mode :type String) (Input%20Media%20Source :type Media%20Source%20Object%20Reference))
  (bind _mp (Variables|Default|GetMP))
  (Variables|Default|SetCurrent%20Media%20Source (stale EventPlayMedia MediaSource))
  (Variables|Default|SetMedia%20Mode "")
  (Media|MediaPlayer|OpenSource _mp 0)
  (EventDispatchers|AssignOnMediaOpened _mp (delegate Custom|OnMediaOpened)))

(event Custom|OnMediaOpened
  (params (OpenedUrl :type String))
  (bind _mp (Variables|Default|GetMP))
  (if (Variables|Default|GetbPlay)
    (Media|MediaPlayer|Play _mp :!class /Script/MediaAssets.MediaPlayer)
    (EventDispatchers|AssignOnEndReached _mp (delegate Custom|OnEndReached_Event))))

(event EventBeginPlay)

(event Collision|EventActorBeginOverlap
  (params (OtherActor :type Actor%20Object%20Reference)))

(event EventTick
  (params (DeltaSeconds :type Float%20%28single-precision%29)))

(event EventPlayMedia
  (params (MediaSource :type Media%20Source%20Object%20Reference))
  (bind _mp (Variables|Default|GetMP))
  (Variables|Default|SetCurrent%20Media%20Source MediaSource)
  (Variables|Default|SetMedia%20Mode "")
  (Media|MediaPlayer|OpenSource _mp 0)
  (EventDispatchers|AssignOnMediaOpened _mp (delegate Custom|OnMediaOpened)))

(fn ConstructionScript)