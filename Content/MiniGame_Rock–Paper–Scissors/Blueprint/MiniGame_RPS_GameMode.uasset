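; Game mode for a VR rock-paper-scissors minigame played through 360 videos, from lobby and map selection to victory or game over.
; Each turn pits the player's detected gesture against a random bot pick, retrying missed gestures via FlipFlop before counting an error.
; Player wins advance the round toward victory, while repeated bot wins or errors restart the game.
; Clips come from per-map DataTables, matched by action, round and variant, and play on BP_RPS_360Player.
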(event Custom|Event%20Select%20Map
  (params (Current_Map :type E_Map%20Enum :default "NewEnumerator0"))
  ;[0.3662 0.724 0.3942 0.5 20] Event Map Select
  (bind _output_get (Variables|Current|SetCurrent_Map Current_Map))
  (Utilities|FlowControl|Sequence
    (:then_0
      (Utilities|FlowControl|DoOnce false
        (:Completed
          (Utilities|FlowControl|Delay 1.0)
          (Variables|Current|SetCurrent_GameState "NewEnumerator4"))))
    (:then_1
      (Default|SelectMapEvent (Variables|Default|Get360Player) _output_get))))

(event Custom|Event%20Confirm%20Map
  (bind _current_map (Variables|Current|GetCurrent_Map))
  ;[0.3662 0.724 0.3942 0.5 20] Event Map Select
  (Utilities|FlowControl|Sequence
    (:then_0
      (Variables|Current|SetCurrent_GameState "NewEnumerator5")
      (Class|WidgetComponent|SetDrawSize (Variables|/Game/MiniGame_Rock–Paper–Scissors/Blueprint/MiniGame_RPS_Pawn.MiniGame_RPS_Pawn_C|GetHUD (Variables|Default|GetMini%20Game%20Pawn)) "(X=500.000000,Y=350.000000)")
      (if (not (Variables|Logic|GetbGameStart))
        (Transformation|SetRelativeLocation (Variables|/Game/MiniGame_Rock–Paper–Scissors/Blueprint/MiniGame_RPS_Pawn.MiniGame_RPS_Pawn_C|GetHUD (Variables|Default|GetMini%20Game%20Pawn)) "400.000000,-250.000000,-20.000000" false false)
        (Default|ConfirmMapEvent (Variables|Default|Get360Player))
        (Variables|Logic|SetbGameStart true)))
    (:then_1
      (Variables|Current|SetCurrent_DataTable (Utilities|Array|Get(acopy) (Variables|Media_Data|GetDT_Media) (+ (Math|Conversions|ToInteger(Byte) _current_map) 1)))
      (switch Utilities|FlowControl|Switch|SwitchonE_Map _current_map
        (:NewEnumerator0
          (Variables|Current|SetCurrent_Media_Row_Name (Variables|Media_Data|GetMap01%20Media%20Row%20Name)))
        (:NewEnumerator1
          (Variables|Current|SetCurrent_Media_Row_Name (Variables|Media_Data|GetMap02%20Media%20Row%20Name)))
        (:NewEnumerator2
          (Variables|Current|SetCurrent_Media_Row_Name (Variables|Media_Data|GetMap03%20Media%20Row%20Name))))
      (CallFunction|CallPlayinGameMedia "NewEnumerator4" (Variables|Logic|GetRound) "A" (Variables|Current|GetCurrent_DataTable))
      ;[0.8698 0.1665 0.6143 0.5 20] Event In Game
      (Utilities|FlowControl|DoOnce false) ; enters at Reset
    )))

(event Custom|Event%20Idle
  ;[0.07286 0.485 0.8229 0.5 20] Event Idle
  (Variables|Current|SetCurrent_GameState "NewEnumerator1")
  (Class|WidgetComponent|SetDrawSize (Variables|/Game/MiniGame_Rock–Paper–Scissors/Blueprint/MiniGame_RPS_Pawn.MiniGame_RPS_Pawn_C|GetHUD (Variables|Default|GetMini%20Game%20Pawn)) "(X=400.000000,Y=150.000000)"))

(event Custom|PostGame
  (bind _current_gesture (Variables|Current|GetCurrent_Gesture))
  ;[0.02471 0.2382 0.5938 0.5] Event  Post Game
  (switch Utilities|FlowControl|Switch|SwitchonE_GestureType _current_gesture
    (:NewEnumerator0
      (CallFunction|Calculate (Math|Conversions|ToInteger(Byte) _current_gesture) (Variables|Logic|GetNumRandBot) :!label _label)
      (Development|PrintString (Utilities|String|EnumtoString (Variables|Current|GetCurrent_Gesture)) true true "(R=0.000000,G=0.660000,B=1.000000,A=1.000000)" 1e+01 :!label _label_2)
      (Variables|Current|SetCurrent_GameState "NewEnumerator2")
      (switch string (Variables|Debug|GetResult)
        (:Win
          (Variables|Logic|SetResult_Index 0))
        (:Lose
          (Variables|Logic|SetResult_Index 1))
        (:Draw
          (Variables|Logic|SetResult_Index 2))
        (:Error
          (Variables|Logic|SetResult_Index 3)))
      (CallFunction|CallPlayinGameMedia (Utilities|Select :Index (Variables|Logic|GetResult_Index) :Option%200 "NewEnumerator5" :Option%201 "NewEnumerator6" :Option%202 "NewEnumerator7" :Option%203 "NewEnumerator8") (Variables|Logic|GetRound) (Variables|Current|GetCurrent_MediaVariant) (Variables|Current|GetCurrent_DataTable))
      (Utilities|FlowControl|Delay 3.0)
      (CallFunction|ValidateGameStatus))
    (:NewEnumerator1
      (goto _label))
    (:NewEnumerator2
      (goto _label))
    (:NewEnumerator3
      (Utilities|FlowControl|FlipFlop :!label _label_3
        (:A
          (Utilities|FlowControl|Delay 3.0)
          (CallFunction|PostGame))
        (:B
          (Math|Integer|IncrementInt (Variables|Logic|GetError)
            (:%20%20
              (Variables|Debug|SetResult "Error")
              (goto _label_2))))))
    (:NewEnumerator7
      (goto _label_3))))

(event Custom|Reset
  ;[0.3662 0.724 0.3942 0.5 20] Event Map Select
  (Utilities|FlowControl|DoOnce false) ; enters at Reset
)

(event Custom|Return%20Idle
  ;[0.3662 0.724 0.3942 0.5 20] Event Map Select
  (Variables|Current|SetCurrent_GameState "NewEnumerator5")
  (Class|WidgetComponent|SetDrawSize (Variables|/Game/MiniGame_Rock–Paper–Scissors/Blueprint/MiniGame_RPS_Pawn.MiniGame_RPS_Pawn_C|GetHUD (Variables|Default|GetMini%20Game%20Pawn)) "(X=500.000000,Y=350.000000)")
  (switch Utilities|FlowControl|Switch|SwitchonE_Map (Variables|Current|GetCurrent_Map)
    (:NewEnumerator0
      (Variables|Current|SetCurrent_Media_Row_Name (Variables|Media_Data|GetMap01%20Media%20Row%20Name)))
    (:NewEnumerator1
      (Variables|Current|SetCurrent_Media_Row_Name (Variables|Media_Data|GetMap02%20Media%20Row%20Name)))
    (:NewEnumerator2
      (Variables|Current|SetCurrent_Media_Row_Name (Variables|Media_Data|GetMap03%20Media%20Row%20Name))))
  (CallFunction|CallPlayinGameMedia "NewEnumerator4" (Variables|Logic|GetRound) "A" (Variables|Current|GetCurrent_DataTable))
  ;[0.8698 0.1665 0.6143 0.5 20] Event In Game
  (Utilities|FlowControl|DoOnce false) ; enters at Reset
)

(event Custom|Validate%20Game%20Status
  ;[0.8542 0.02364 0.09169 0.5 30] Game Rule Validate
  ;;[0.15 0.15 0.15 0.5] Lose or Error >= 3 times
  (if (>= (Variables|Logic|GetBotWin) 3)
    (Variables|Current|SetCurrent_GameState "NewEnumerator3" :!label _label)
    (Variables|Debug|SetDebug_Current_Media (Utilities|String|ToString(Text) (Utilities|Text|FormatText "GameOver 
Try Again!!!")))
    (Utilities|FlowControl|Delay 5.0)
    (CallFunction|Restart)
    (elif (== (Variables|Logic|GetError) 3)
      (goto _label)
      (elif (== (Variables|Logic|GetRound) 9)
        (Variables|Current|SetCurrent_GameState "NewEnumerator3")
        (CallFunction|CallPlayinGameMedia "NewEnumerator9" (Variables|Logic|GetRound) (Variables|Current|GetCurrent_MediaVariant) (Variables|Current|GetCurrent_DataTable))
        (Utilities|FlowControl|Delay 5.0)
        (Variables|Debug|SetDebug_Current_Media (Utilities|String|ToString(Text) (Utilities|Text|FormatText "Victory")))
        (Utilities|FlowControl|Delay 5.0)
        (CallFunction|Restart :!pinned true) ; Restart
        (else
          (switch string (Variables|Debug|GetResult)
            (:Win
              (CallFunction|CallPlayinGameMedia "NewEnumerator9" (Variables|Logic|GetRound) (Variables|Current|GetCurrent_MediaVariant) (Variables|Current|GetCurrent_DataTable))
              (Utilities|FlowControl|Delay 1e+01))
            (:Lose
              (Utilities|FlowControl|Delay 1.0 :!label _label_2))
            (:Draw
              (goto _label_2))
            (:Error
              (goto _label_2)))
          (CallFunction|ReturnIdle :!pinned true) ; Return to Idle
        )))))

(event Custom|Event%20%20Action
  ;[0.8698 0.1665 0.6143 0.5 20] Event In Game
  (Rendering|SetVisibility (Variables|/Game/MiniGame_Rock–Paper–Scissors/Blueprint/MiniGame_RPS_Pawn.MiniGame_RPS_Pawn_C|GetHUD (Variables|Default|GetMini%20Game%20Pawn)) true true)
  (bind _output_get (Variables|Logic|SetNumRandBot (Math|Random|RandomIntegerinRange 0 2)))
  (CallFunction|CallPlayinGameMedia (Utilities|Select :Index _output_get :Option%200 "NewEnumerator1" :Option%201 "NewEnumerator2" :Option%202 "NewEnumerator3") (Variables|Logic|GetRound) (Variables|Current|GetCurrent_MediaVariant) (Variables|Current|GetCurrent_DataTable))
  (Utilities|FlowControl|Delay 5.0)
  (Rendering|SetVisibility (Variables|/Game/MiniGame_Rock–Paper–Scissors/Blueprint/MiniGame_RPS_Pawn.MiniGame_RPS_Pawn_C|GetHUD (Variables|Default|GetMini%20Game%20Pawn)) true true)
  (Utilities|FlowControl|Delay 1.0)
  (CallFunction|PostGame))

(event EventBeginPlay
  ;[1 1 1 0.5 40] Event Begin Play
  (Utilities|FlowControl|Sequence
    (:then_0
      (Development|ExecuteConsoleCommand "stereo on" 0 :!pinned true) ; Command for VR Gameplay
    )
    (:then_1
      (Utilities|FlowControl|DoOnce false
        (:Completed
          ;;[0.05547 0.7656 0.3795 0.5] Set Media Data Variables
          (for (_array_element _array_index) (Variables|Media_Data|GetDT_Media)
            (bind _outrownames (DataTable|GetDataTableRowNames _array_element))
            (switch int _array_index
              (:0
                (Variables|Media_Data|SetMain%20Media%20Row%20Name _outrownames))
              (:1
                (Variables|Media_Data|SetMap01%20Media%20Row%20Name _outrownames))
              (:2
                (Variables|Media_Data|SetMap02%20Media%20Row%20Name _outrownames))
              (:3
                (Variables|Media_Data|SetMap03%20Media%20Row%20Name _outrownames))))
          ;;[0.05547 0.7656 0.3795 0.5] Set Actor & Pawn Variables
          (bind _returnvalue (Actor|GetActorOfClass "/Game/MiniGame_Rock–Paper–Scissors/Blueprint/BP_RPS_360Player.BP_RPS_360Player_C"))
          (Variables|Default|Set360Player _returnvalue)
          (bind _asmini_game_rps_pawn (Utilities|Casting|CastToMiniGame_RPS_Pawn (Game|Player|GetPlayerPawn 0)))
          (Variables|Default|SetMini%20Game%20Pawn _asmini_game_rps_pawn))))
    (:then_2
      (Utilities|FlowControl|Sequence
        (:then_0
          ;;[0.7292 0.1519 0.1519 0.5] Reset Game Logic Variable
          (Transformation|SetRelativeLocation (Variables|/Game/MiniGame_Rock–Paper–Scissors/Blueprint/MiniGame_RPS_Pawn.MiniGame_RPS_Pawn_C|GetHUD (Variables|Default|GetMini%20Game%20Pawn)) "400.000000,0.000000,-20.000000" false false)
          (Class|WidgetComponent|SetDrawSize (Variables|/Game/MiniGame_Rock–Paper–Scissors/Blueprint/MiniGame_RPS_Pawn.MiniGame_RPS_Pawn_C|GetHUD (Variables|Default|GetMini%20Game%20Pawn)) "(X=500.000000,Y=350.000000)"))
        (:then_1
          (Variables|Current|SetCurrent_GameState "NewEnumerator0"))
        (:then_2
          (Variables|Logic|SetRound 0))
        (:then_3
          (Variables|Logic|SetbGameStart false))
        (:then_4
          (Variables|Logic|SetBotWin 0))
        (:then_5
          (Variables|Logic|SetError 0))
        (:then_6
          (Variables|Current|SetCurrent_Map "NewEnumerator0"))))
    (:then_3
      (CallFunction|PlayLobbyMedia :!pinned true) ; Play Lobby Media
    )))

(event EventGestureChange
  (params (Gesture%20Type%20Detect :type E_GestureType%20Enum :default "NewEnumerator0"))
  ;[0.8698 0.1665 0.6143 0.5 20] Event In Game
  (Variables|Current|SetCurrent_Gesture Gesture%20Type%20Detect)
  (Utilities|FlowControl|DoOnce false
    (:Completed
      (CallFunction|EventAction))))

(event EventRestart
  ;[1 1 1 0.5 40] Event Begin Play
  ;;[0.1437 0.2266 0.4271 0.5] Restart Game
  (Default|Restart (Variables|Default|Get360Player))
  (CallFunction|Reset)
  (Utilities|FlowControl|Sequence
    (:then_0
      (Development|ExecuteConsoleCommand "stereo on" 0 :!pinned true) ; Command for VR Gameplay
    )
    (:then_1
      (Utilities|FlowControl|DoOnce false
        (:Completed
          ;;[0.05547 0.7656 0.3795 0.5] Set Media Data Variables
          (for (_array_element _array_index) (Variables|Media_Data|GetDT_Media)
            (bind _outrownames (DataTable|GetDataTableRowNames _array_element))
            (switch int _array_index
              (:0
                (Variables|Media_Data|SetMain%20Media%20Row%20Name _outrownames))
              (:1
                (Variables|Media_Data|SetMap01%20Media%20Row%20Name _outrownames))
              (:2
                (Variables|Media_Data|SetMap02%20Media%20Row%20Name _outrownames))
              (:3
                (Variables|Media_Data|SetMap03%20Media%20Row%20Name _outrownames))))
          ;;[0.05547 0.7656 0.3795 0.5] Set Actor & Pawn Variables
          (bind _returnvalue (Actor|GetActorOfClass "/Game/MiniGame_Rock–Paper–Scissors/Blueprint/BP_RPS_360Player.BP_RPS_360Player_C"))
          (Variables|Default|Set360Player _returnvalue)
          (bind _asmini_game_rps_pawn (Utilities|Casting|CastToMiniGame_RPS_Pawn (Game|Player|GetPlayerPawn 0)))
          (Variables|Default|SetMini%20Game%20Pawn _asmini_game_rps_pawn))))
    (:then_2
      (Utilities|FlowControl|Sequence
        (:then_0
          ;;[0.7292 0.1519 0.1519 0.5] Reset Game Logic Variable
          (Transformation|SetRelativeLocation (Variables|/Game/MiniGame_Rock–Paper–Scissors/Blueprint/MiniGame_RPS_Pawn.MiniGame_RPS_Pawn_C|GetHUD (Variables|Default|GetMini%20Game%20Pawn)) "400.000000,0.000000,-20.000000" false false)
          (Class|WidgetComponent|SetDrawSize (Variables|/Game/MiniGame_Rock–Paper–Scissors/Blueprint/MiniGame_RPS_Pawn.MiniGame_RPS_Pawn_C|GetHUD (Variables|Default|GetMini%20Game%20Pawn)) "(X=500.000000,Y=350.000000)"))
        (:then_1
          (Variables|Current|SetCurrent_GameState "NewEnumerator0"))
        (:then_2
          (Variables|Logic|SetRound 0))
        (:then_3
          (Variables|Logic|SetbGameStart false))
        (:then_4
          (Variables|Logic|SetBotWin 0))
        (:then_5
          (Variables|Logic|SetError 0))
        (:then_6
          (Variables|Current|SetCurrent_Map "NewEnumerator0"))))
    (:then_3
      (CallFunction|PlayLobbyMedia :!pinned true) ; Play Lobby Media
    )))

(fn ConstructionScript)

(fn RequestMedia
  (for _array_element (Variables|Media_Data|GetMain%20Media%20Row%20Name)
    _))

(fn CallPlayMainMedia
  (params (Media%20Type :type E_MediaType%20Enum :default "NewEnumerator0"))
  (for _array_element (Variables|Media_Data|GetMain%20Media%20Row%20Name)
    (bind _returnvalue (Utilities|GetDataTableRow (Utilities|Array|Get(acopy) (Variables|Media_Data|GetDT_Media)) _array_element)
      (:then
        (if (and (Utilities|Enum|Equal(Enum) (Variables|Current|GetCurrent_Map) (.Map (Utilities|Struct|BreakST_Data_Media _returnvalue))) (Utilities|Enum|Equal(Enum) (.MediaType (Utilities|Struct|BreakST_Data_Media _returnvalue)) Media%20Type))
          (bind _output_get (Variables|Debug|SetMedia%20Name _array_element))
          (bind _output_get_2 (Variables|Current|SetCurrent_MediaSource (.MediaSource (Utilities|Struct|BreakST_Data_Media _returnvalue))))
          (bind _output_get_3 (Variables|Debug|SetDebug_Current_Media (Utilities|String|ToString(Text) (Utilities|Text|FormatText "Round: {R} 
Media: {Media} 
Map: {M}" (Variables|Logic|GetRound) _output_get (Utilities|String|EnumtoString (Variables|Current|GetCurrent_Map))))))
          (Default|PlayMedia (Variables|Default|Get360Player) _output_get_2 _output_get_3))))))

(fn Calculate
  (params (InputNumPlayer :type Integer) (Input_NumRandBot :type Integer))
  (bind _output_get (LocalVariables|SetNum_Player InputNumPlayer))
  (bind _output_get_2 (LocalVariables|SetNum_Rand_Bot Input_NumRandBot))
  (if (== _output_get _output_get_2)
    (Variables|Debug|SetResult "Draw")
    (elif (Math|Boolean|ORBoolean (and (== (LocalVariables|GetNum_Player) 0) (== (LocalVariables|GetNum_Rand_Bot) 2)) (and (== (LocalVariables|GetNum_Player) 1) (== (LocalVariables|GetNum_Rand_Bot) 0)) (and (== (LocalVariables|GetNum_Player) 2) (== (LocalVariables|GetNum_Rand_Bot) 1)))
      (Variables|Debug|SetResult "Win")
      (Math|Integer|IncrementInt (Variables|Logic|GetRound))
      (else
        (Variables|Debug|SetResult "Lose")
        (Math|Integer|IncrementInt (Variables|Logic|GetBotWin))))))

(fn CallPlayinGameMedia
  (params (Input%20Action :type E_Bot_Action%20Enum :default "NewEnumerator0") (Round :type Integer) (Media%20Variant :type String) (CurrentDataTable :type Data%20Table%20Object%20Reference))
  (for _array_element (Variables|Current|GetCurrent_Media_Row_Name)
    (bind _returnvalue (Utilities|GetDataTableRow CurrentDataTable _array_element)
      (:then
        (if (Math|Boolean|ANDBoolean (Utilities|Enum|Equal(Enum) (.Action (Utilities|Struct|BreakST_Map_Media _returnvalue)) Input%20Action) (== (.Round (Utilities|Struct|BreakST_Map_Media _returnvalue)) Round) (Utilities|Enum|Equal(Enum) (.MediaVariant (Utilities|Struct|BreakST_Map_Media _returnvalue)) Media%20Variant))
          (bind _output_get (Variables|Debug|SetMedia%20Name _array_element))
          (bind _output_get_2 (Variables|Current|SetCurrent_MediaSource (.Media_Source (Utilities|Struct|BreakST_Map_Media _returnvalue))))
          (bind _output_get_3 (Variables|Debug|SetDebug_Current_Media (Utilities|String|ToString(Text) (Utilities|Text|FormatText "Round: {R} 
Media: {Media} 
Map: {M}" (Variables|Logic|GetRound) _output_get (Utilities|String|EnumtoString (Variables|Current|GetCurrent_Map))))))
          (Default|PlayMedia (Variables|Default|Get360Player) _output_get_2 _output_get_3))))))

(fn PlayLobbyMedia
  (for _array_element (Variables|Media_Data|GetMain%20Media%20Row%20Name)
    (bind _returnvalue (Utilities|GetDataTableRow (Utilities|Array|Get(acopy) (Variables|Media_Data|GetDT_Media)) _array_element)
      (:then
        (switch Utilities|FlowControl|Switch|SwitchonE_MediaType (.MediaType (Utilities|Struct|BreakST_Data_Media _returnvalue))
          (:NewEnumerator5
            (bind _output_get (Variables|Current|SetCurrent_MediaSource (.MediaSource (Utilities|Struct|BreakST_Data_Media _returnvalue))))
            (Default|PlayMedia (Variables|Default|Get360Player) _output_get (Utilities|String|EnumtoString (.MediaType (Utilities|Struct|BreakST_Data_Media _returnvalue))))))))))

(fn PlayMedia
  (params (MediaSource :type Media%20Source%20Object%20Reference) (MediaMode :type String))
  (return))