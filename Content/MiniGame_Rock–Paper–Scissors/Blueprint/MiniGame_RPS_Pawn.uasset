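; Player pawn for the Rock-Paper-Scissors minigame that turns XR hand tracking into gestures.
; Each Tick it picks detectors by game mode state, measuring hand socket distances to read thumbs-up menu gestures or rock, paper and scissors.
; Gesture changes are sent to the player controller, and repeated failed in-game reads set a separate error gesture.
; Enhanced Input actions emulate gestures for editor testing, alongside debug prints and a state-driven debug display.
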(event Input|EnhancedActionEvents|EnhancedInputActionIA_Restart
  (params (ActionValue :type Float%20%28double-precision%29) (ElapsedSeconds :type Float%20%28double-precision%29) (TriggeredSeconds :type Float%20%28double-precision%29) (InputAction :type Input%20Action%20Object%20Reference :default "/Game/MiniGame_Rock–Paper–Scissors/Input/IA_Restart.IA_Restart"))
  ;[0 0 0] Play in Editor Debug
  (Class|BPIRPSGameFlow|Restart(Message) (Game|GetGameMode)))

(event Input|EnhancedActionEvents|EnhancedInputActionIA_Start
  (params (ActionValue :type Float%20%28double-precision%29) (ElapsedSeconds :type Float%20%28double-precision%29) (TriggeredSeconds :type Float%20%28double-precision%29) (InputAction :type Input%20Action%20Object%20Reference :default "/Game/MiniGame_Rock–Paper–Scissors/Input/IA_Start.IA_Start"))
  ;[0 0 0] Play in Editor Debug
  (Variables|Default|SetCurrentGesture "NewEnumerator4")
  (switch Utilities|FlowControl|Switch|SwitchonE_GameState (Variables|/Game/MiniGame_Rock–Paper–Scissors/Blueprint/MiniGame_RPS_GameMode.MiniGame_RPS_GameMode_C|GetCurrent_GameState (Variables|Default|GetRPS%20Game%20Mode))
    (:NewEnumerator0
      (Utilities|FlowControl|Delay 0.1 :!label _label)
      (Variables|Default|SetCurrentGesture "NewEnumerator3"))
    (:NewEnumerator4
      (goto _label))
    (:NewEnumerator5
      (Variables|Default|SetbErrorDetect true))))

(event Input|EnhancedActionEvents|EnhancedInputActionIA_Next
  (params (ActionValue :type Float%20%28double-precision%29) (ElapsedSeconds :type Float%20%28double-precision%29) (TriggeredSeconds :type Float%20%28double-precision%29) (InputAction :type Input%20Action%20Object%20Reference :default "/Game/MiniGame_Rock–Paper–Scissors/Input/IA_Next.IA_Next"))
  ;[0 0 0] Play in Editor Debug
  (Variables|Default|SetCurrentGesture "NewEnumerator5")
  (Utilities|FlowControl|Delay 0.1)
  (Variables|Default|SetCurrentGesture "NewEnumerator3"))

(event Input|EnhancedActionEvents|EnhancedInputActionIA_Back
  (params (ActionValue :type Float%20%28double-precision%29) (ElapsedSeconds :type Float%20%28double-precision%29) (TriggeredSeconds :type Float%20%28double-precision%29) (InputAction :type Input%20Action%20Object%20Reference :default "/Game/MiniGame_Rock–Paper–Scissors/Input/IA_Back.IA_Back"))
  ;[0 0 0] Play in Editor Debug
  (Variables|Default|SetCurrentGesture "NewEnumerator6")
  (Utilities|FlowControl|Delay 0.1)
  (Variables|Default|SetCurrentGesture "NewEnumerator3"))

(event Input|EnhancedActionEvents|EnhancedInputActionIA_Rock
  (params (ActionValue :type Float%20%28double-precision%29) (ElapsedSeconds :type Float%20%28double-precision%29) (TriggeredSeconds :type Float%20%28double-precision%29) (InputAction :type Input%20Action%20Object%20Reference :default "/Game/MiniGame_Rock–Paper–Scissors/Input/IA_Rock.IA_Rock"))
  ;[0 0 0] Play in Editor Debug
  (Variables|Default|SetCurrentGesture "NewEnumerator0"))

(event Input|EnhancedActionEvents|EnhancedInputActionIA_Paper
  (params (ActionValue :type Float%20%28double-precision%29) (ElapsedSeconds :type Float%20%28double-precision%29) (TriggeredSeconds :type Float%20%28double-precision%29) (InputAction :type Input%20Action%20Object%20Reference :default "/Game/MiniGame_Rock–Paper–Scissors/Input/IA_Paper.IA_Paper"))
  ;[0 0 0] Play in Editor Debug
  (Variables|Default|SetCurrentGesture "NewEnumerator1"))

(event Input|EnhancedActionEvents|EnhancedInputActionIA_Scissors
  (params (ActionValue :type Float%20%28double-precision%29) (ElapsedSeconds :type Float%20%28double-precision%29) (TriggeredSeconds :type Float%20%28double-precision%29) (InputAction :type Input%20Action%20Object%20Reference :default "/Game/MiniGame_Rock–Paper–Scissors/Input/IA_Scissors.IA_Scissors"))
  ;[0 0 0] Play in Editor Debug
  (Variables|Default|SetCurrentGesture "NewEnumerator2"))

(event EventBeginPlay
  (Input|AddMappingContext (PlayerController|LocalPlayerSubsystems|GetEnhancedInputLocalPlayerSubsystem (Game|GetPlayerController 0)) "/Game/MiniGame_Rock–Paper–Scissors/Input/IMC_MiniGame.IMC_MiniGame" 0 "(bIgnoreAllPressedKeysUntilRelease=True,bForceImmediately=False,bNotifyUserSettings=False)")
  ;[0.15 0.15 0.15 0.5] Set Gamemode Variable
  (bind _asmini_game_rps_game_mode (Utilities|Casting|CastToMiniGame_RPS_GameMode (Game|GetGameMode)))
  (bind _output_get (Variables|Default|SetRPS%20Game%20Mode _asmini_game_rps_game_mode))
  (bind _asw_rps_mini_game (Utilities|Casting|CastToW_RPS_MiniGame (UserInterface|GetWidget (Variables|Default|GetHUD))))
  (Variables|/Game/MiniGame_Rock–Paper–Scissors/Blueprint/W_RPS_MiniGame.W_RPS_MiniGame_C|SetRPS%20Game%20Mode _asw_rps_mini_game _output_get))

(event Collision|EventActorBeginOverlap
  (params (OtherActor :type Actor%20Object%20Reference)))

(event EventTick
  (params (DeltaSeconds :type Float%20%28single-precision%29))
  (Utilities|FlowControl|Sequence
    (:then_0
      (CallFunction|FNDetectGesture :!pinned true) ; Detect Gesture
    )
    (:then_1
      (CallFunction|FNDebugGesture))
    (:then_2
      (CallFunction|DebugFinger))
    (:then_3
      ;[0 0.03034 0.15 0.5] Clear Gesture
      (if (Math|Boolean|ORBoolean (Utilities|Enum|Equal(Enum) (Variables|Default|GetCurrentGesture) "NewEnumerator4") (Utilities|Enum|Equal(Enum) (Variables|Default|GetCurrentGesture) "NewEnumerator5") (Utilities|Enum|Equal(Enum) (Variables|Default|GetCurrentGesture) "NewEnumerator6"))
        (Utilities|FlowControl|Delay 0.5)
        (Variables|Default|SetCurrentGesture "NewEnumerator3")))))

(fn ConstructionScript)

(fn FNDetectGesture
  (Utilities|FlowControl|Sequence
    (:then_0
      (switch Utilities|FlowControl|Switch|SwitchonE_GameState (Variables|/Game/MiniGame_Rock–Paper–Scissors/Blueprint/MiniGame_RPS_GameMode.MiniGame_RPS_GameMode_C|GetCurrent_GameState (Variables|Default|GetRPS%20Game%20Mode))
        (:NewEnumerator0
          (CallFunction|FNHandtrackBeforeGameStart :!label _label))
        (:NewEnumerator4
          (goto _label))
        (:NewEnumerator5
          (bind _return_confirm (CallFunction|FNDetectConfirm))
          (if _return_confirm
            (Variables|Default|SetCurrentGesture "NewEnumerator4")
            (Variables|Default|SetbErrorDetect true)))
        (:NewEnumerator1
          (CallFunction|FNDetectinGame :!pinned true) ; Detect in Gameplay
        )))
    (:then_1
      (if (Utilities|Enum|NotEqual(Enum) (Variables|Default|GetCurrentGesture) (Variables|Default|GetPreviousGesture))
        (bind _output_get (Variables|Default|SetPreviousGesture (Variables|Default|GetCurrentGesture)))
        (bind _asmini_game_rps_controller (Utilities|Casting|CastToMiniGame_RPS_Controller (Pawn|GetController)))
        (Class|BPIRPSInput|GestureChange(Message) _asmini_game_rps_controller _output_get)))))

(fn FNDetectPaper
  (bind _bp_xrhandcomponent_right (Variables|Default|GetBP_XRHandComponent_Right))
  (bind _distance_between_the_thumb_and_little (Variables|Messure_Value|GetDistance%20between%20the%20thumb%20and%20little))
  (bind _distance_from_the_index_tip_to_the_base (Variables|Messure_Value|GetDistance%20from%20the%20index%20tip%20to%20the%20base))
  (bind _bp_xrhandcomponent_right_2 (Variables|Default|GetBP_XRHandComponent_Right))
  (bind _returnvalue (Transformation|GetSocketTransform _bp_xrhandcomponent_right "right_thumb_tip" "RTS_World"))
  (bind _returnvalue_2 (Transformation|GetSocketTransform _bp_xrhandcomponent_right "right_little_tip" "RTS_World"))
  (bind _returnvalue_3 (Transformation|GetSocketTransform _bp_xrhandcomponent_right_2 "right_index_proximal" "RTS_World"))
  (bind _returnvalue_4 (Transformation|GetSocketTransform _bp_xrhandcomponent_right_2 "right_index_tip" "RTS_World"))
  (bind _location (Math|Transform|BreakTransform _returnvalue_3))
  (bind _location_2 (Math|Transform|BreakTransform _returnvalue_4))
  (bind _location_3 (Math|Transform|BreakTransform _returnvalue))
  (bind _location_4 (Math|Transform|BreakTransform _returnvalue_2))
  (bind _returnvalue_5 (- _location_2 _location))
  (bind _returnvalue_6 (- _location_3 _location_4))
  (bind _returnvalue_7 (Math|Vector|VectorLength _returnvalue_5))
  (bind _returnvalue_8 (Math|Vector|VectorLength _returnvalue_6))
  (bind _returnvalue_9 (> _returnvalue_7 _distance_from_the_index_tip_to_the_base))
  (bind _returnvalue_10 (> _returnvalue_8 _distance_between_the_thumb_and_little))
  (bind _returnvalue_11 (and _returnvalue_10 _returnvalue_9))
  (if _returnvalue_11
    (Development|PrintString "Player: Paper" true true "(R=0.000000,G=0.660000,B=1.000000,A=1.000000)" 2.0 "P")
    (return _returnvalue_11)))

(fn FNDetectScissors
  (bind _bp_xrhandcomponent_right (Variables|Default|GetBP_XRHandComponent_Right))
  (bind _bp_xrhandcomponent_right_2 (Variables|Default|GetBP_XRHandComponent_Right))
  (bind _bp_xrhandcomponent_right_3 (Variables|Default|GetBP_XRHandComponent_Right))
  (bind _returnvalue (Transformation|GetSocketTransform _bp_xrhandcomponent_right "right_index_tip" "RTS_World"))
  (bind _returnvalue_2 (Transformation|GetSocketTransform _bp_xrhandcomponent_right "right_palm" "RTS_World"))
  (bind _returnvalue_3 (Transformation|GetSocketTransform _bp_xrhandcomponent_right_3 "right_thumb_tip" "RTS_World"))
  (bind _returnvalue_4 (Transformation|GetSocketTransform _bp_xrhandcomponent_right_3 "right_palm" "RTS_World"))
  (bind _returnvalue_5 (Transformation|GetSocketTransform _bp_xrhandcomponent_right_2 "right_middle_tip" "RTS_World"))
  (bind _returnvalue_6 (Transformation|GetSocketTransform _bp_xrhandcomponent_right_2 "right_palm" "RTS_World"))
  (bind _location (Math|Transform|BreakTransform _returnvalue_3))
  (bind _location_2 (Math|Transform|BreakTransform _returnvalue_4))
  (bind _location_3 (Math|Transform|BreakTransform _returnvalue))
  (bind _location_4 (Math|Transform|BreakTransform _returnvalue_2))
  (bind _location_5 (Math|Transform|BreakTransform _returnvalue_5))
  (bind _location_6 (Math|Transform|BreakTransform _returnvalue_6))
  (bind _returnvalue_7 (- _location_3 _location_4))
  (bind _returnvalue_8 (- _location_5 _location_6))
  (bind _returnvalue_9 (- _location _location_2))
  (bind _returnvalue_10 (Math|Vector|VectorLength _returnvalue_9))
  (bind _returnvalue_11 (Math|Vector|VectorLength _returnvalue_7))
  (bind _returnvalue_12 (Math|Vector|VectorLength _returnvalue_8))
  (bind _returnvalue_13 (> _returnvalue_11 9.0))
  (bind _returnvalue_14 (> _returnvalue_12 9.0))
  (bind _returnvalue_15 (< _returnvalue_10 8.0))
  (bind _returnvalue_16 (Math|Boolean|ANDBoolean _returnvalue_13 _returnvalue_15 _returnvalue_14))
  (if _returnvalue_16
    (Development|PrintString "Player: Scissors" true true "(R=0.000000,G=0.660000,B=1.000000,A=1.000000)" 2.0 "S")
    (return _returnvalue_16)))

(fn FNHandtrackBeforeGameStart
  (bind _return_confirm (CallFunction|FNDetectConfirm))
  (if _return_confirm
    (Variables|Default|SetCurrentGesture "NewEnumerator4")
    (else
      (bind _return_condition (CallFunction|FNDetectNext))
      (if _return_condition
        (Utilities|FlowControl|FlipFlop
          (:A
            (Variables|Default|SetCurrentGesture "NewEnumerator5"))
          (:B
            (Variables|Default|SetCurrentGesture "NewEnumerator3")))
        (else
          (bind _return_condition_2 (CallFunction|FNDetectBack))
          (if _return_condition_2
            (Utilities|FlowControl|FlipFlop
              (:A
                (Variables|Default|SetCurrentGesture "NewEnumerator6"))
              (:B
                (Variables|Default|SetCurrentGesture "NewEnumerator3")))))))))

(fn FNDetectConfirm
  (bind _bp_xrhandcomponent_right (Variables|Default|GetBP_XRHandComponent_Right))
  (bind _bp_xrhandcomponent_left (Variables|Default|GetBP_XRHandComponent_Left))
  (bind _bp_xrhandcomponent_left_2 (Variables|Default|GetBP_XRHandComponent_Left))
  (bind _bp_xrhandcomponent_right_2 (Variables|Default|GetBP_XRHandComponent_Right))
  (bind _returnvalue (Transformation|GetSocketTransform _bp_xrhandcomponent_left "left_thumb_tip" "RTS_World"))
  (bind _returnvalue_2 (Transformation|GetSocketTransform _bp_xrhandcomponent_left "left_palm" "RTS_World"))
  (bind _returnvalue_3 (Transformation|GetSocketTransform _bp_xrhandcomponent_right "right_index_tip" "RTS_World"))
  (bind _returnvalue_4 (Transformation|GetSocketTransform _bp_xrhandcomponent_right "right_palm" "RTS_World"))
  (bind _returnvalue_5 (Transformation|GetSocketTransform _bp_xrhandcomponent_left_2 "left_palm" "RTS_World"))
  (bind _returnvalue_6 (Transformation|GetSocketTransform _bp_xrhandcomponent_left_2 "left_index_tip" "RTS_World"))
  (bind _returnvalue_7 (Transformation|GetSocketTransform _bp_xrhandcomponent_right_2 "right_thumb_tip" "RTS_World"))
  (bind _returnvalue_8 (Transformation|GetSocketTransform _bp_xrhandcomponent_right_2 "right_palm" "RTS_World"))
  (bind _location (Math|Transform|BreakTransform _returnvalue_3))
  (bind _location_2 (Math|Transform|BreakTransform _returnvalue_4))
  (bind _location_3 (Math|Transform|BreakTransform _returnvalue_5))
  (bind _location_4 (Math|Transform|BreakTransform _returnvalue_6))
  (bind _location_5 (Math|Transform|BreakTransform _returnvalue))
  (bind _location_6 (Math|Transform|BreakTransform _returnvalue_7))
  (bind _location_7 (Math|Transform|BreakTransform _returnvalue_8))
  (bind _location_8 (Math|Transform|BreakTransform _returnvalue_2))
  (bind _returnvalue_9 (- _location_4 _location_3))
  (bind _returnvalue_10 (- _location_5 _location_8))
  (bind _returnvalue_11 (- _location_6 _location_7))
  (bind _returnvalue_12 (- _location _location_2))
  (bind _returnvalue_13 (Math|Vector|VectorLength _returnvalue_12))
  (bind _returnvalue_14 (Math|Vector|VectorLength _returnvalue_9))
  (bind _returnvalue_15 (Math|Vector|VectorLength _returnvalue_11))
  (bind _returnvalue_16 (Math|Vector|VectorLength _returnvalue_10))
  (bind _returnvalue_17 (< _returnvalue_14 5.0))
  (bind _returnvalue_18 (> _returnvalue_15 9.0))
  (bind _returnvalue_19 (> _returnvalue_16 9.0))
  (bind _returnvalue_20 (< _returnvalue_13 5.0))
  (bind _returnvalue_21 (and _returnvalue_18 _returnvalue_20))
  (bind _returnvalue_22 (and _returnvalue_19 _returnvalue_17))
  (bind _returnvalue_23 (and _returnvalue_21 _returnvalue_22))
  (Development|PrintString (Utilities|String|ToString(Boolean) _returnvalue_23) true true "(R=0.000000,G=0.660000,B=1.000000,A=1.000000)" 2.0 "D")
  (if _returnvalue_23
    (return _returnvalue_23)))

(fn FNDetectNext
  (bind _bp_xrhandcomponent_right (Variables|Default|GetBP_XRHandComponent_Right))
  (bind _bp_xrhandcomponent_right_2 (Variables|Default|GetBP_XRHandComponent_Right))
  (bind _returnvalue (Transformation|GetSocketTransform _bp_xrhandcomponent_right "right_index_tip" "RTS_World"))
  (bind _returnvalue_2 (Transformation|GetSocketTransform _bp_xrhandcomponent_right "right_palm" "RTS_World"))
  (bind _returnvalue_3 (Transformation|GetSocketTransform _bp_xrhandcomponent_right_2 "right_thumb_tip" "RTS_World"))
  (bind _returnvalue_4 (Transformation|GetSocketTransform _bp_xrhandcomponent_right_2 "right_palm" "RTS_World"))
  (bind _location (Math|Transform|BreakTransform _returnvalue))
  (bind _location_2 (Math|Transform|BreakTransform _returnvalue_2))
  (bind _location_3 (Math|Transform|BreakTransform _returnvalue_3))
  (bind _location_4 (Math|Transform|BreakTransform _returnvalue_4))
  (bind _returnvalue_5 (- _location_3 _location_4))
  (bind _returnvalue_6 (- _location _location_2))
  (bind _returnvalue_7 (Math|Vector|VectorLength _returnvalue_6))
  (bind _returnvalue_8 (Math|Vector|VectorLength _returnvalue_5))
  (bind _returnvalue_9 (> _returnvalue_8 9.0))
  (bind _returnvalue_10 (< _returnvalue_7 5.0))
  (bind _returnvalue_11 (and _returnvalue_9 _returnvalue_10))
  (if _returnvalue_11
    (return _returnvalue_11)))

(fn FNDetectBack
  (bind _bp_xrhandcomponent_left (Variables|Default|GetBP_XRHandComponent_Left))
  (bind _bp_xrhandcomponent_left_2 (Variables|Default|GetBP_XRHandComponent_Left))
  (bind _returnvalue (Transformation|GetSocketTransform _bp_xrhandcomponent_left "left_thumb_tip" "RTS_World"))
  (bind _returnvalue_2 (Transformation|GetSocketTransform _bp_xrhandcomponent_left "left_palm" "RTS_World"))
  (bind _returnvalue_3 (Transformation|GetSocketTransform _bp_xrhandcomponent_left_2 "left_palm" "RTS_World"))
  (bind _returnvalue_4 (Transformation|GetSocketTransform _bp_xrhandcomponent_left_2 "left_index_tip" "RTS_World"))
  (bind _location (Math|Transform|BreakTransform _returnvalue_3))
  (bind _location_2 (Math|Transform|BreakTransform _returnvalue_4))
  (bind _location_3 (Math|Transform|BreakTransform _returnvalue))
  (bind _location_4 (Math|Transform|BreakTransform _returnvalue_2))
  (bind _returnvalue_5 (- _location_2 _location))
  (bind _returnvalue_6 (- _location_3 _location_4))
  (bind _returnvalue_7 (Math|Vector|VectorLength _returnvalue_5))
  (bind _returnvalue_8 (Math|Vector|VectorLength _returnvalue_6))
  (bind _returnvalue_9 (< _returnvalue_7 5.0))
  (bind _returnvalue_10 (> _returnvalue_8 9.0))
  (bind _returnvalue_11 (and _returnvalue_10 _returnvalue_9))
  (if _returnvalue_11
    (return _returnvalue_11)))

(fn FNDetectRock
  (bind _bp_xrhandcomponent_right (Variables|Default|GetBP_XRHandComponent_Right))
  (bind _bp_xrhandcomponent_right_2 (Variables|Default|GetBP_XRHandComponent_Right))
  (bind _bp_xrhandcomponent_right_3 (Variables|Default|GetBP_XRHandComponent_Right))
  (bind _bp_xrhandcomponent_right_4 (Variables|Default|GetBP_XRHandComponent_Right))
  (bind _returnvalue (Transformation|GetSocketTransform _bp_xrhandcomponent_right "right_middle_tip" "RTS_World"))
  (bind _returnvalue_2 (Transformation|GetSocketTransform _bp_xrhandcomponent_right "right_palm" "RTS_World"))
  (bind _returnvalue_3 (Transformation|GetSocketTransform _bp_xrhandcomponent_right_3 "right_little_tip" "RTS_World"))
  (bind _returnvalue_4 (Transformation|GetSocketTransform _bp_xrhandcomponent_right_3 "right_palm" "RTS_World"))
  (bind _returnvalue_5 (Transformation|GetSocketTransform _bp_xrhandcomponent_right_4 "right_thumb_tip" "RTS_World"))
  (bind _returnvalue_6 (Transformation|GetSocketTransform _bp_xrhandcomponent_right_4 "right_palm" "RTS_World"))
  (bind _returnvalue_7 (Transformation|GetSocketTransform _bp_xrhandcomponent_right_2 "right_index_tip" "RTS_World"))
  (bind _returnvalue_8 (Transformation|GetSocketTransform _bp_xrhandcomponent_right_2 "right_palm" "RTS_World"))
  (bind _location (Math|Transform|BreakTransform _returnvalue_3))
  (bind _location_2 (Math|Transform|BreakTransform _returnvalue_4))
  (bind _location_3 (Math|Transform|BreakTransform _returnvalue))
  (bind _location_4 (Math|Transform|BreakTransform _returnvalue_5))
  (bind _location_5 (Math|Transform|BreakTransform _returnvalue_6))
  (bind _location_6 (Math|Transform|BreakTransform _returnvalue_2))
  (bind _location_7 (Math|Transform|BreakTransform _returnvalue_7))
  (bind _location_8 (Math|Transform|BreakTransform _returnvalue_8))
  (bind _returnvalue_9 (- _location_3 _location_6))
  (bind _returnvalue_10 (- _location_7 _location_8))
  (bind _returnvalue_11 (- _location_4 _location_5))
  (bind _returnvalue_12 (- _location _location_2))
  (bind _returnvalue_13 (Math|Vector|VectorLength _returnvalue_12))
  (bind _returnvalue_14 (Math|Vector|VectorLength _returnvalue_11))
  (bind _returnvalue_15 (Math|Vector|VectorLength _returnvalue_9))
  (bind _returnvalue_16 (Math|Vector|VectorLength _returnvalue_10))
  (bind _returnvalue_17 (< _returnvalue_14 8.5))
  (bind _returnvalue_18 (< _returnvalue_15 6.0))
  (bind _returnvalue_19 (< _returnvalue_16 6.0))
  (bind _returnvalue_20 (< _returnvalue_13 6.0))
  (bind _returnvalue_21 (Math|Boolean|ANDBoolean _returnvalue_17 _returnvalue_19 _returnvalue_20 _returnvalue_18))
  (if _returnvalue_21
    (return _returnvalue_21)))

(fn FNDebugGesture
  (switch Utilities|FlowControl|Switch|SwitchonE_GameState (Variables|/Game/MiniGame_Rock–Paper–Scissors/Blueprint/MiniGame_RPS_GameMode.MiniGame_RPS_GameMode_C|GetCurrent_GameState (Variables|Default|GetRPS%20Game%20Mode))
    (:NewEnumerator0
      (LocalVariables|SetbTemp false :!label _label))
    (:NewEnumerator4
      (goto _label))
    (:NewEnumerator5
      (goto _label))
    (:NewEnumerator1
      (LocalVariables|SetbTemp true :!label _label_2))
    (:NewEnumerator2
      (goto _label_2))
    (:NewEnumerator3
      (goto _label)))
  (if (!= (LocalVariables|GetbTemp) (Rendering|IsVisible (Variables|Default|GetDebug)))
    (Rendering|SetVisibility (Variables|Default|GetDebug) (LocalVariables|GetbTemp) false)))

(fn DebugFinger
  (bind _bp_xrhandcomponent_right (Variables|Default|GetBP_XRHandComponent_Right))
  (bind _returnvalue (Transformation|GetSocketTransform _bp_xrhandcomponent_right "right_palm" "RTS_World"))
  (bind _location (Math|Transform|BreakTransform _returnvalue))
  (Development|PrintString (Utilities|String|ToString(Text) (Utilities|Text|FormatText "Thumb: {T} 
Index: {I} 
Middle: {M} 
Ring: {R} 
Little: {L}" (Math|Vector|VectorLength (- (.Location (Math|Transform|BreakTransform (Transformation|GetSocketTransform _bp_xrhandcomponent_right "right_thumb_tip" "RTS_World"))) _location)) (Math|Vector|VectorLength (- (.Location (Math|Transform|BreakTransform (Transformation|GetSocketTransform _bp_xrhandcomponent_right "right_index_tip" "RTS_World"))) _location)) (Math|Vector|VectorLength (- (.Location (Math|Transform|BreakTransform (Transformation|GetSocketTransform _bp_xrhandcomponent_right "right_middle_tip" "RTS_World"))) _location)) (Math|Vector|VectorLength (- (.Location (Math|Transform|BreakTransform (Transformation|GetSocketTransform _bp_xrhandcomponent_right "right_ring_tip" "RTS_World"))) _location)) (Math|Vector|VectorLength (- (.Location (Math|Transform|BreakTransform (Transformation|GetSocketTransform _bp_xrhandcomponent_right "right_little_tip" "RTS_World"))) _location)))) true true "(R=1.000000,G=0.248225,B=0.000000,A=1.000000)" 2.0 "Measure"))

(fn FNDetectinGame
  (bind _returncondition (CallFunction|FNDetectPaper :!pinned true)) ; Paper
  (if _returncondition
    (Variables|Default|SetCurrentGesture "NewEnumerator1")
    (LocalVariables|SetErrorCount 0)
    (Variables|Default|SetbErrorDetect true)
    (else
      (bind _return_condition (CallFunction|FNDetectScissors :!pinned true)) ; Scissors
      (if _return_condition
        (Variables|Default|SetCurrentGesture "NewEnumerator2")
        (LocalVariables|SetErrorCount 0)
        (Variables|Default|SetbErrorDetect true)
        (else
          (bind _return_condition_2 (CallFunction|FNDetectRock :!pinned true)) ; Rock
          (if _return_condition_2
            (Variables|Default|SetCurrentGesture "NewEnumerator0")
            (LocalVariables|SetErrorCount 0)
            (Variables|Default|SetbErrorDetect true)
            (elif (and (Variables|Default|GetbErrorDetect) (>= (LocalVariables|GetErrorCount) 50))
              (Variables|Default|SetCurrentGesture "NewEnumerator7")
              (Variables|Default|SetbErrorDetect false)
              (elif (Variables|Default|GetbErrorDetect)
                (bind _result (Math|Integer|IncrementInt (LocalVariables|GetErrorCount))
                  (:%20%20
                    (LocalVariables|SetErrorCount _result)))))))))))