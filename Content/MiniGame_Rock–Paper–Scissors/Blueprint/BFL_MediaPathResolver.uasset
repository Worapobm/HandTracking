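; Blueprint function library for the Rock-Paper-Scissors minigame that resolves a video ID to an MP4 file path for media playback.
; ResolveMediaPath switches on platform name: Windows builds the path under the project's ExternalMedia/Movies folder.
; Android and every other platform use a hard-coded external app-storage Movies path tied to the package name.
; Some leftover user-directory path nodes are unused.
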(fn ResolveMediaPath
  (params (VideoID :type String))
  (switch string (Game|GetPlatformName)
    (:Default
      _)
    (:Android
      _)
    (:Windows
      (return (Utilities|String|Append (Utilities|String|Append (Utilities|String|Append (Class|KismetSystemLibrary|GetProjectDirectory) "ExternalMedia/Movies/") VideoID) ".mp4"))))
  (return (Utilities|String|Append (Utilities|String|Append "/storage/emulated/0/Android/data/com.VerseX.minigame_rockpaperscissors/files/Movies/" VideoID) ".mp4")))