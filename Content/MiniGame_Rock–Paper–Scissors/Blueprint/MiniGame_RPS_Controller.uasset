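; Controller for the Rock–Paper–Scissors minigame that turns detected gestures into game mode actions.
; It caches the RPS game mode on BeginPlay and routes each gesture change by the current game state.
; Start/Confirm advances Lobby, Map Select and Idle, while Next and Back step through the map enum using modulo on the entry count.
; In Game forwards the gesture straight to the game mode.
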(event EventBeginPlay
  ;[0.15 0.15 0.15 0.5] Promote Gamemode
  (bind _asmini_game_rps_game_mode (Utilities|Casting|CastToMiniGame_RPS_GameMode (Game|GetGameMode)))
  (Variables|Default|SetRPS%20Game%20Mode _asmini_game_rps_game_mode))

(event EventTick
  (params (DeltaSeconds :type Float%20%28single-precision%29)))

(event EventGestureChange
  (params (Gesture%20Type%20Detect :type E_GestureType%20Enum :default "NewEnumerator0"))
  (bind _rps_game_mode (Variables|Default|GetRPS%20Game%20Mode))
  (bind _current_map (Variables|/Game/MiniGame_Rock–Paper–Scissors/Blueprint/MiniGame_RPS_GameMode.MiniGame_RPS_GameMode_C|GetCurrent_Map _rps_game_mode))
  (bind _returnvalue (Math|Conversions|ToInteger(Byte) _current_map))
  (Variables|Default|SetGesture%20Type%20Detect Gesture%20Type%20Detect)
  (switch Utilities|FlowControl|Switch|SwitchonE_GameState (Variables|/Game/MiniGame_Rock–Paper–Scissors/Blueprint/MiniGame_RPS_GameMode.MiniGame_RPS_GameMode_C|GetCurrent_GameState (Variables|Default|GetRPS%20Game%20Mode))
    (:NewEnumerator0
      (switch Utilities|FlowControl|Switch|SwitchonE_GestureType (Variables|Default|GetGesture%20Type%20Detect)
        (:NewEnumerator4
          (Default|EventSelectMap (Variables|Default|GetRPS%20Game%20Mode) "NewEnumerator0"))))
    (:NewEnumerator4
      (switch Utilities|FlowControl|Switch|SwitchonE_GestureType (Variables|Default|GetGesture%20Type%20Detect)
        (:NewEnumerator4
          (Default|EventConfirmMap (Variables|Default|GetRPS%20Game%20Mode)))
        (:NewEnumerator5
          ;[0.3651 0.3671 0.6198 0.5] Event Select Map
          (Variables|Default|SetbPick true)
          (bind _result (Math|Integer|IncrementInt _returnvalue)
            (:%20%20
              (Default|EventSelectMap (Variables|Default|GetRPS%20Game%20Mode) (Utilities|Select :Index (Utilities|Enum|ByteToEnumE_Map (Math|Conversions|ToByte(Integer) (Math|Integer|%(Integer) (Math|Integer|SelectInt _result (stale _result_2) (Variables|Default|GetbPick)) (|GetNumEnumEntries)))) :NewEnumerator0 "NewEnumerator0" :NewEnumerator1 "NewEnumerator1" :NewEnumerator2 "NewEnumerator2" :NewEnumerator3 "NewEnumerator0") :!label _label))))
        (:NewEnumerator6
          (Variables|Default|SetbPick false)
          (bind _result_2 (Math|Integer|DecrementInt _returnvalue)
            (:%20%20
              (goto _label))))))
    (:NewEnumerator5
      (switch Utilities|FlowControl|Switch|SwitchonE_GestureType (Variables|Default|GetGesture%20Type%20Detect)
        (:NewEnumerator4
          (Default|EventIdle (Variables|Default|GetRPS%20Game%20Mode)))))
    (:NewEnumerator1
      (Default|GestureChange (Variables|Default|GetRPS%20Game%20Mode) (Variables|Default|GetGesture%20Type%20Detect)))))

(fn ConstructionScript)