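; 360 media player actor for the Rock-Paper-Scissors minigame, showing video or a map preview on a dome mesh.
; PlayMedia opens a source on the media player, plays it once opened if Play is set, and reopens it on end to loop.
; A dynamic dome material blends to the selected map's texture via SwitchMedia, switched once per selection phase.
; Confirming a map or restarting sets SwitchMedia back; restarting also re-arms the DoOnce.
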(event Custom|SelectMap_Event
  (params (Input%20Current%20Map :type E_Map%20Enum :default "NewEnumerator0"))
  (bind _mid (Variables|Default|GetMID))
  ;[0.3662 0.724 0.3942 0.5] Map Select
  (Utilities|FlowControl|Sequence
    (:then_0
      (Utilities|FlowControl|DoOnce false
        (:Completed
          (Rendering|Material|SetScalarParameterValue _mid "SwitchMedia" 1.0 :!class /Script/Engine.MaterialInstanceDynamic))))
    (:then_1
      (Rendering|Material|SetTextureParameterValue _mid "Map" (Utilities|Select :Index Input%20Current%20Map :NewEnumerator0 "/Game/StarterContent/Textures/T_Wood_Oak_D.T_Wood_Oak_D" :NewEnumerator1 "/Game/StarterContent/Textures/T_Wood_Pine_D.T_Wood_Pine_D" :NewEnumerator2 "/Game/StarterContent/Textures/T_Metal_Aluminum_D.T_Metal_Aluminum_D" :NewEnumerator3 0)))))

(event Custom|ConfirmMap_Event
  ;[0.3662 0.724 0.3942 0.5] Map Select
  (Rendering|Material|SetScalarParameterValue (Variables|Default|GetMID) "SwitchMedia" 0.0 :!class /Script/Engine.MaterialInstanceDynamic))

(event Custom|OnEndReached_Event
  (bind _current_media_source (Variables|Default|GetCurrent%20Media%20Source))
  ;[0.7083 0.214 0.214 0.5] Play Media Loop
  (Media|MediaPlayer|OpenSource (Variables|Default|GetMP) _current_media_source)
  (CallFunction|PlayMediaSourceLoop (Variables|Default|GetMedia%20Mode) _current_media_source :!pinned true) ; Play Loop
)

(event Custom|Play%20Media%20Source%20Loop
  (params (Media%20Mode :type String) (Input%20Media%20Source :type Media%20Source%20Object%20Reference))
  (bind _mp (Variables|Default|GetMP))
  ;[0.7083 0.214 0.214 0.5] Play Media Loop
  (Media|MediaPlayer|OpenSource _mp (stale EventPlayMedia _output_get))
  (EventDispatchers|AssignOnMediaOpened _mp (delegate Custom|OnMediaOpened) :!pinned true) ; Check Media Open Completely
)

(event Custom|Reset
  ;[0.3662 0.724 0.3942 0.5] Map Select
  (Utilities|FlowControl|DoOnce false) ; enters at Reset
)

(event Custom|OnMediaOpened
  (params (OpenedUrl :type String))
  (bind _mp (Variables|Default|GetMP))
  ;[0.7083 0.214 0.214 0.5] Play Media Loop
  (if (Variables|Default|GetbPlay)
    (Media|MediaPlayer|Play _mp :!class /Script/MediaAssets.MediaPlayer)
    (EventDispatchers|AssignOnEndReached _mp (delegate Custom|OnEndReached_Event) :!pinned true) ; Check Media End Completely
  ))

(event EventBeginPlay
  (bind _sm_dome (Variables|Default|GetSM_Dome))
  (bind _returnvalue (Rendering|Material|CreateDynamicMaterialInstance _sm_dome 0 (Rendering|Material|GetMaterial _sm_dome 0) "None" :!class /Script/Engine.PrimitiveComponent))
  (Variables|Default|SetMID _returnvalue))

(event EventTick
  (params (DeltaSeconds :type Float%20%28single-precision%29)))

(event EventRestart
  (CallFunction|Reset)
  (Rendering|Material|SetScalarParameterValue (Variables|Default|GetMID) "SwitchMedia" 0.0 :!class /Script/Engine.MaterialInstanceDynamic))

(event EventPlayMedia
  (params (MediaSource :type Media%20Source%20Object%20Reference) (MediaMode :type String))
  (bind _mp (Variables|Default|GetMP))
  ;[0.7083 0.214 0.214 0.5] Play Media Loop
  (bind _output_get (Variables|Default|SetCurrent%20Media%20Source MediaSource))
  (Variables|Default|SetMedia%20Mode MediaMode)
  (Media|MediaPlayer|OpenSource _mp _output_get)
  (EventDispatchers|AssignOnMediaOpened _mp (delegate Custom|OnMediaOpened) :!pinned true) ; Check Media Open Completely
)

(fn ConstructionScript)